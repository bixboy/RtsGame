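; RTS player Blueprint that maps Enhanced Input actions to movement, zoom, rotation, selection and command functions defined outside this graph.
; Press and release events drive rotation toggling, left and right mouse selection, and commands.
; The delete action passes the RTS controller's selected actors to ServerDestroy, which destroys each one.
; RotateLeft and RotateRight calls are disconnected, so their input actions do nothing.
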(event `EnhancedInput|/Game/BP/Input/IA/IA_Move`
  (params (ActionValue :type "Float (double-precision)") (ElapsedSeconds :type "Float (double-precision)") (TriggeredSeconds :type "Float (double-precision)") (InputAction :type "InputAction Object Reference" :default "/Game/BP/Input/IA/IA_Move.IA_Move"))
  ;[0.2066 1 0.9502] Movement
  (:`Triggered`
    (`self.MoveForward` ActionValue)))

(event `EnhancedInput|/Game/BP/Input/IA/IA_Zoom`
  (params (ActionValue :type "Float (double-precision)") (ElapsedSeconds :type "Float (double-precision)") (TriggeredSeconds :type "Float (double-precision)") (InputAction :type "InputAction Object Reference" :default "/Game/BP/Input/IA/IA_Zoom.IA_Zoom"))
  ;[0.2066 1 0.9502] Movement
  (:`Triggered`
    (`self.Zoom` ActionValue)))

(event `EnhancedInput|/Game/BP/Input/IA/IA_MoveRight`
  (params (ActionValue :type "Float (double-precision)") (ElapsedSeconds :type "Float (double-precision)") (TriggeredSeconds :type "Float (double-precision)") (InputAction :type "InputAction Object Reference" :default "/Game/BP/Input/IA/IA_MoveRight.IA_MoveRight"))
  ;[0.2066 1 0.9502] Movement
  (:`Triggered`
    (`self.MoveRight` ActionValue)))

(event `EnhancedInput|/Game/BP/Input/IA/IA_Rotate`
  (params (ActionValue :type Boolean) (ElapsedSeconds :type "Float (double-precision)") (TriggeredSeconds :type "Float (double-precision)") (InputAction :type "InputAction Object Reference" :default "/Game/BP/Input/IA/IA_Rotate.IA_Rotate"))
  ;[0.717 1 0.2545] Rotation
  (:`Started`
    (`self.EnableRotation`))
  (:`Completed`
    (`self.DisableRotation`)))

(event `EnhancedInput|/Game/BP/Input/IA/IA_RotateHorizontal`
  (params (ActionValue :type "Float (double-precision)") (ElapsedSeconds :type "Float (double-precision)") (TriggeredSeconds :type "Float (double-precision)") (InputAction :type "InputAction Object Reference" :default "/Game/BP/Input/IA/IA_RotateHorizontal.IA_RotateHorizontal"))
  ;[0.717 1 0.2545] Rotation
  (:`Triggered`
    (`self.RotateHorizontal` ActionValue)))

(event `EnhancedInput|/Game/BP/Input/IA/IA_RotateRight`
  (params (ActionValue :type Boolean) (ElapsedSeconds :type "Float (double-precision)") (TriggeredSeconds :type "Float (double-precision)") (InputAction :type "InputAction Object Reference" :default "/Game/BP/Input/IA/IA_RotateRight.IA_RotateRight"))
  ;[0.717 1 0.2545] Rotation
)

(event `EnhancedInput|/Game/BP/Input/IA/IA_RotateVertical`
  (params (ActionValue :type "Float (double-precision)") (ElapsedSeconds :type "Float (double-precision)") (TriggeredSeconds :type "Float (double-precision)") (InputAction :type "InputAction Object Reference" :default "/Game/BP/Input/IA/IA_RotateVertical.IA_RotateVertical"))
  ;[0.717 1 0.2545] Rotation
  (:`Triggered`
    (`self.RotateVertical` ActionValue)))

(event `EnhancedInput|/Game/BP/Input/IA/IA_RotateLeft`
  (params (ActionValue :type Boolean) (ElapsedSeconds :type "Float (double-precision)") (TriggeredSeconds :type "Float (double-precision)") (InputAction :type "InputAction Object Reference" :default "/Game/BP/Input/IA/IA_RotateLeft.IA_RotateLeft"))
  ;[0.717 1 0.2545] Rotation
)

(event `EnhancedInput|/Game/BP/Input/IA/IA_Select`
  (params (ActionValue :type Boolean) (ElapsedSeconds :type "Float (double-precision)") (TriggeredSeconds :type "Float (double-precision)") (InputAction :type "InputAction Object Reference" :default "/Game/BP/Input/IA/IA_Select.IA_Select"))
  ;[1 0.177 0.187] Selection
  (:`Started`
    (`self.LeftMousePressed`))
  (:`Completed`
    (`self.LeftMouseReleased`)))

(event `EnhancedInput|/Game/BP/Input/IA/IA_DeSelect`
  (params (ActionValue :type Boolean) (ElapsedSeconds :type "Float (double-precision)") (TriggeredSeconds :type "Float (double-precision)") (InputAction :type "InputAction Object Reference" :default "/Game/BP/Input/IA/IA_DeSelect.IA_DeSelect"))
  ;[1 0.177 0.187] Selection
  (:`Started`
    (`self.RightMousePressed`))
  (:`Completed`
    (`self.RightMouseReleased`)))

(event `EnhancedInput|/Game/BP/Input/IA/IA_SelectTrigger`
  (params (ActionValue :type "Float (double-precision)") (ElapsedSeconds :type "Float (double-precision)") (TriggeredSeconds :type "Float (double-precision)") (InputAction :type "InputAction Object Reference" :default "/Game/BP/Input/IA/IA_SelectTrigger.IA_SelectTrigger"))
  ;[1 0.177 0.187] Selection
  (:`Triggered`
    (`self.LeftMouseInputHold` ActionValue)))

(event `EnhancedInput|/Game/BP/Input/IA/IA_Command`
  (params (ActionValue :type Boolean) (ElapsedSeconds :type "Float (double-precision)") (TriggeredSeconds :type "Float (double-precision)") (InputAction :type "InputAction Object Reference" :default "/Game/BP/Input/IA/IA_Command.IA_Command"))
  (:`Started`
    (`self.CommandStart`))
  (:`Completed`
    (`self.Command`)))

(event `EnhancedInput|/Game/BP/Input/IA/IA_Delete`
  (params (ActionValue :type Boolean) (ElapsedSeconds :type "Float (double-precision)") (TriggeredSeconds :type "Float (double-precision)") (InputAction :type "InputAction Object Reference" :default "/Game/BP/Input/IA/IA_Delete.IA_Delete"))
  (bind _returnvalue (`PlayerControllerRts.GetSelectedActors` (`self.GetRtsPlayerController`)))
  (:`Started`
    (if (> (`KismetArrayLibrary.Array_Length` _returnvalue) 0)
      (`self.ServerDestroy` _returnvalue))))

(event `ServerDestroy`
  (params (Array :type "Array of Actor Object Reference"))
  (for _array_element Array
    (`self.K2_DestroyActor` _array_element)))

(fn `UserConstructionScript`)